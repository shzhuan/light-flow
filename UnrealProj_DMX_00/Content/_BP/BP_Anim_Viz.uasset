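; BP_Anim_Viz is a visualizer actor that plays a scale animation on a sphere when TriggerAnim is called.
; The construction script applies the Material variable to the sphere and starts it at a small scale.
; TriggerAnim restarts the Anim01 timeline, whose Alpha drives the sphere's uniform relative scale, with the play rate sped up on BeginPlay.
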(event Custom|TriggerAnim
  (bind _alpha (Timeline|Anim01 PlayFromStart)
    (:Update
      (Transformation|SetRelativeScale3D (Variables|Default|GetSphere) (Math|Conversions|ToVector(Float) _alpha)))))

(event EventBeginPlay
  (Components|Timeline|SetPlayRate (Variables|Default|GetAnim01) 3.0))

(fn ConstructionScript
  (Rendering|Material|SetMaterial (Variables|Default|GetSphere) 0 (Variables|Default|GetMaterial))
  (Transformation|SetRelativeScale3D (Variables|Default|GetSphere) "0.100000,0.100000,0.100000"))