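; BP_LaserM2 is an actor Blueprint that sends DMX data to a fixture from DMXLibrary_01, apparently as a laser control test.
; On BeginPlay it caches the library's fixtures and prints the first one's name.
; SendDmxf plays a timeline, printing each value and sending it truncated as a single-channel map to that first fixture.
; GetGameData and SpawnFixtureActors are empty stubs, and the construction script only builds an unused map.
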(event EventBeginPlay
  (CallFunction|UpdateActorVariables self)
  (bind _returnvalue (Class|DMXSubsystem|GetAllFixturesinLibrary (|DMXSubsystem) "/Game/DMX/DMXLibrary_01.DMXLibrary_01"))
  (Development|PrintString (Utilities|GetDisplayName (Utilities|Array|Get(acopy) _returnvalue))))

(event Collision|EventActorBeginOverlap
  (params (OtherActor :type Actor%20Object%20Reference)))

(event EventTick
  (params (DeltaSeconds :type Float%20%28single-precision%29)))

(event EventSendDmxf
  (params (NewParam :type Integer) (DmxAttrMap :type Map%20of%20DMX%20Attribute%20Name%20Structures%20to%20Integers))
  (bind _newtrack_0 (Timeline|Timeline PlayFromStart)
    (:Update
      (Development|PrintString (Utilities|String|ToString(Float) _newtrack_0))
      (bind _output_get (Variables|Default|SetChannels (Utilities|Map|MakeMap "(Name=\"OnOff\")" (Math|Float|Truncate _newtrack_0) "(Name=\"Zoom\")" 0 "(Name=\"PatternGrp\")" 0 "(Name=\"PatternSel\")" 0 "(Name=\"ZoomAnim\")" 0 "(Name=\"Rotate\")" 0 "(Name=\"Pan\")" 0 "(Name=\"Tilt\")" 0 "(Name=\"ScaleX\")" 0 "(Name=\"ScaleY\")" 0 "(Name=\"ColorFlow\")" 0 "(Name=\"Color\")" 0 "(Name=\"Segments\")" 0 "(Name=\"Draw\")" 0 "(Name=\"AutoDraw\")" 0 "(Name=\"Undefined\")" 0 "(Name=\"Shrink\")" 0 "(Name=\"OnOff_00\")" 0 "(Name=\"Zoom_00\")" 0 "(Name=\"PatternGrp_00\")" 0 "(Name=\"PatternSel_00\")" 0 "(Name=\"ZoomAnim_00\")" 0 "(Name=\"Rotate_00\")" 0 "(Name=\"Pan_00\")" 0 "(Name=\"Tilt_00\")" 0 "(Name=\"ScaleX_00\")" 0 "(Name=\"ScaleY_00\")" 0 "(Name=\"ColorFlow_00\")" 0 "(Name=\"Color_00\")" 0 "(Name=\"Segments_00\")" 0 "(Name=\"Draw_00\")" 0 "(Name=\"AutoDraw_00\")" 0 "(Name=\"Undefined_00\")" 0 "(Name=\"Shrink_00\")" 0)))
      (Class|DMXEntityFixturePatch|SendDMX (Utilities|Array|Get(acopy) (stale EventBeginPlay _returnvalue)) _output_get))))

(fn ConstructionScript
  (Variables|Default|SetChannels (Utilities|Map|MakeMap "(Name=\"OnOff\")" 0 "(Name=\"Zoom\")" 0 "(Name=\"PatternGrp\")" 0 "(Name=\"PatternSel\")" 0 "(Name=\"ZoomAnim\")" 0 "(Name=\"Rotate\")" 0 "(Name=\"Pan\")" 0 "(Name=\"Tilt\")" 0 "(Name=\"ScaleX\")" 0 "(Name=\"ScaleY\")" 0 "(Name=\"ColorFlow\")" 0 "" 0 "(Name=\"Segments\")" 0 "(Name=\"Draw\")" 0 "(Name=\"AutoDraw\")" 0 "(Name=\"Undefined\")" 0 "(Name=\"Shrink\")" 0 "(Name=\"OnOff_00\")" 0 "(Name=\"Zoom_00\")" 0 "(Name=\"PatternGrp_00\")" 0 "(Name=\"PatternSel_00\")" 0 "(Name=\"ZoomAnim_00\")" 0 "(Name=\"Rotate_00\")" 0 "(Name=\"Pan_00\")" 0 "(Name=\"Tilt_00\")" 0 "(Name=\"ScaleX_00\")" 0 "(Name=\"ScaleY_00\")" 0 "(Name=\"ColorFlow_00\")" 0 "(Name=\"Color_00\")" 0 "(Name=\"Segments_00\")" 0 "(Name=\"Draw_00\")" 0 "(Name=\"AutoDraw_00\")" 0 "(Name=\"Undefined_00\")" 0 "(Name=\"Shrink_00\")" 0)))

(fn GetGameData
  (return 0))

(fn SpawnFixtureActors
  (params (FixtureNames :type Text))
  (return 0 0 0))