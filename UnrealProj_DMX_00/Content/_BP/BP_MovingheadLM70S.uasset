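; Actor that controls an LM70S moving-head DMX light, using the fixture at index 1 of a DMX library.
; BeginPlay fetches the fixtures, and custom events send channel maps, store color and strobe, or stop and zero output.
; SendPlayRate runs a ping-pong timeline that re-enters the send path each update, though the map built from its lerp, color and strobe is unconnected.
; GetPlayerSave exposes channels and fade timings; UsePlayerSave is empty.
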(event Custom|OnCHValueChanged_Event
  (params (ChannelValue :type Integer) (dmxAttrName :type DMX%20Attribute%20Name%20Structure)))

(event EventBeginPlay
  (CallFunction|UpdateActorVariables self)
  (bind _returnvalue (Class|DMXSubsystem|GetAllFixturesinLibrary (|DMXSubsystem) "/Game/DMX/DMXLibrary_01.DMXLibrary_01"))
  (Development|PrintString (Utilities|GetDisplayName (Utilities|Array|Get(acopy) _returnvalue 1)))
  (Class|DMXEntityFixturePatch|SendDMX (Utilities|Array|Get(acopy) _returnvalue 1) (Utilities|Map|MakeMap "(Name=\"Pan\")" 0 "(Name=\"Tilt\")" 0 "(Name=\"MasterControl\")" 0 "(Name=\"Red\")" 0 "(Name=\"Green\")" 0 "(Name=\"Blue\")" 0 "(Name=\"White\")" 0 "(Name=\"Velocity\")" 0 "(Name=\"Reset\")" 0)))

(event Collision|EventActorBeginOverlap
  (params (OtherActor :type Actor%20Object%20Reference)))

(event EventTick
  (params (DeltaSeconds :type Float%20%28single-precision%29)))

(event EventSendPlayRate
  (params (Speed :type Float%20%28double-precision%29))
  (Components|Timeline|SetPlayRate (Variables|Default|GetTL_Pingpong) Speed)
  (bind _pingpong (Timeline|TL_Pingpong Play)
    (:Update
      (Development|PrintString (Utilities|String|ToString(Byte) (.R (Math|Color|BreakColor (Variables|Default|GetColor)))))
      (bind _output_get (Variables|Default|SetChannels (stale EventSendDmxf DmxAttrMap)))
      (Class|DMXEntityFixturePatch|SendDMX (Utilities|Array|Get(acopy) (stale EventBeginPlay _returnvalue) 1) _output_get))))

(event EventSendStrobe
  (params (Strobe :type Float%20%28double-precision%29))
  (Variables|Default|SetStrobe Strobe))

(event EventSendDmxf
  (params (NewParam :type Integer) (DmxAttrMap :type Map%20of%20DMX%20Attribute%20Name%20Structures%20to%20Integers))
  (Development|PrintString (Utilities|String|ToString(Byte) (.R (Math|Color|BreakColor (Variables|Default|GetColor)))))
  (bind _output_get (Variables|Default|SetChannels DmxAttrMap))
  (Class|DMXEntityFixturePatch|SendDMX (Utilities|Array|Get(acopy) (stale EventBeginPlay _returnvalue) 1) _output_get))

(event EventSendZero
  (Utilities|FlowControl|Sequence
    (:then_0
      (bind _pingpong (Timeline|TL_Pingpong Stop)
        (:Update
          (Development|PrintString (Utilities|String|ToString(Byte) (.R (Math|Color|BreakColor (Variables|Default|GetColor)))))
          (bind _output_get (Variables|Default|SetChannels (stale EventSendDmxf DmxAttrMap)))
          (Class|DMXEntityFixturePatch|SendDMX (Utilities|Array|Get(acopy) (stale EventBeginPlay _returnvalue) 1) _output_get))))
    (:then_1
      (Class|DMXEntityFixturePatch|SendDMX (Utilities|Array|Get(acopy) (stale EventBeginPlay _returnvalue) 1) (Utilities|Map|MakeMap "(Name=\"Pan\")" 0 "(Name=\"Tilt\")" 0 "(Name=\"MasterControl\")" 0 "(Name=\"Red\")" 0 "(Name=\"Green\")" 0 "(Name=\"Blue\")" 0 "(Name=\"White\")" 0 "(Name=\"Velocity\")" 0 "(Name=\"Reset\")" 0)))))

(event EventSendColor
  (params (LightColor :type Color%20Structure))
  (Variables|Default|SetColor LightColor))

(fn ConstructionScript
  (Variables|Default|SetChannels (Utilities|Map|MakeMap "(Name=\"Pan\")" 0 "(Name=\"Tilt\")" 0 "(Name=\"MasterControl\")" 0 "(Name=\"Red\")" 0 "(Name=\"Green\")" 0 "(Name=\"Blue\")" 0 "(Name=\"White\")" 0 "(Name=\"Velocity\")" 0 "(Name=\"Reset\")" 0)))

(fn UsePlayerSave
  (params (PlayerSave :type S%20Player%20Save%20Structure)))

(fn GetPlayerSave
  (return (Utilities|Struct|MakeS_PlayerSave "" (Variables|Default|GetChannels) (Variables|Default|GetFadeIn) (Variables|Default|GetDuration) (Variables|Default|GetFadeOut) (Variables|Default|GetHold))))