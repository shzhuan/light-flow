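; BP_OSC_01 receives OSC messages and uses them to trigger drum-named animation visualizers.
; On BeginPlay it creates a listening OSC server on a configurable IP and port and binds a message-received event.
; OSC_In stores each message and switches on its address path, calling TriggerAnim on the matching BPAnimVizRef array entry for kick, snare or hihat.
; Two helper functions read the stored message's first argument as an integer or string.
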(event Custom|OSC_In
  (params (Message :type OSC%20Message%20Structure%20%28by%20ref%29) (IPAddress :type String) (Port :type Integer))
  (bind _output_get (Variables|Default|SetOSC_MSG Message))
  (bind _returnvalue (Class|OSCManager|GetOSCMessageAddress _output_get))
  (bind _returnvalue_2 (Class|OSCManager|GetOSCAddressFullPath _returnvalue))
  (switch string _returnvalue_2
    (:/kick
      (Default|TriggerAnim (Utilities|Array|Get(acopy) (Variables|Default|GetBP_AnimVizRef))))
    (:/snare
      (Default|TriggerAnim (Utilities|Array|Get(acopy) (Variables|Default|GetBP_AnimVizRef) 1)))
    (:/hihat
      (Default|TriggerAnim (Utilities|Array|Get(acopy) (Variables|Default|GetBP_AnimVizRef) 2)))))

(event EventBeginPlay
  (bind _returnvalue (Class|OSCManager|CreateOSCServer (Variables|Default|GetReceive%20IPAddress) (Variables|Default|GetPort) false true "" 0))
  (bind _output_get (Variables|Default|SetOSC_Server _returnvalue))
  (EventDispatchers|BindEventtoOnOscMessageReceived _output_get (EventDispatchers|CreateEvent :!event Custom|OSC_In)))

(fn ConstructionScript)

(fn GetIntValue
  (bind _value (Class|OSCManager|GetInt32 (Variables|Default|GetOSC_MSG)))
  (return _value))

(fn GetStrValue
  (bind _value (Class|OSCManager|GetString (Variables|Default|GetOSC_MSG)))
  (return _value))